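; Wind turbine actor that visualizes live MQTT data and highlights its base through custom depth on cursor hover.
; Construction script sets height, rotor size, logo, dirtiness, offshore base and random rotor angle and speed variation.
; Tick parses the MQTT handler's JSON; when total power is present, it shows it, spins rotor and anemometer, and refreshes cost, per-turbine power and failure metrics into a data map and UI.
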(event `self.ReceiveBeginPlay`
  (add `self.OnBeginCursorOver` (delegate `On Mouse Hover`))
  (add `self.OnEndCursorOver` (delegate `On Mouse Hover End`))
  (`KismetSystemLibrary.ExecuteConsoleCommand` "PXVIS COIIISION" null)
  (set `self.Cont Ref_0` (cast `/Game/FirstPerson/Blueprints/BP_FirstPersonCharacter` (`GameplayStatics.GetPlayerCharacter` 0) :!pure true))
  (bind _outactors (`GameplayStatics.GetAllActorsOfClass` "/Game/Blueprints/BP_MQTT_Handler.BP_MQTT_Handler_C"))
  (set `self.MQTT Handler` (`|GetArrayItem` _outactors))
  (bind _returnvalue (* (stale `self.ReceiveTick` DeltaSeconds) (`self.RPM`) -6.0 (+ (* (`self.random_speed_change`) (`KismetMathLibrary.Conv_BoolToDouble` (`self.RPM Variation`))) 1.0)))
  ;[1 1 1] Add rotation to turbine
  (`SceneComponent.K2_AddLocalRotation` (`self.Rotor`) (`KismetMathLibrary.MakeRotator` 0.0 _returnvalue) false false :!label _label)
  (`SceneComponent.K2_AddLocalRotation` (`self.Anemometer`) (`KismetMathLibrary.MakeRotator` 0.0 0.0 (* 5 _returnvalue)) false false)
  ;[1 1 1] Instantiate data
  (`self.Get Turbine Cost`)
  (`self.Get Turbine Power`)
  (`self.Get Moring Line Failure`)
  (`self.Get Tower Buckling`)
  (`self.Get Blade Root Bending`))

(event `On Mouse Hover End` :!signature `self.OnEndCursorOver`
  (params (TouchedActor :type "Actor Object Reference"))
  (`PrimitiveComponent.SetRenderCustomDepth` (`self.Base`) false))

(event `On Mouse Hover` :!signature `self.OnBeginCursorOver`
  (params (TouchedActor :type "Actor Object Reference"))
  (`PrimitiveComponent.SetRenderCustomDepth` (`self.Base`) true))

(event `self.ReceiveTick`
  (params (DeltaSeconds :type "Float (single-precision)"))
  ;[1 1 1] Data from mqtt
  (bind (_outjsonobject _returnvalue) (`JsonBlueprintFunctionLibrary.FromString` (`/Game/Blueprints/BP_MQTT_Handler.Message` (`self.MQTT Handler`))))
  (if _returnvalue
    (bind (_outvalue _returnvalue_2) (`|GetJsonField` _outjsonobject (`KismetStringLibrary.Concat_StrStr` "Total" " " "Power")))
    (if _returnvalue_2
      (`KismetSystemLibrary.PrintString` _outvalue false false (struct :`R` 1.0 :`G` 0.992648 :`B` 0.117468 :`A` 1.0) 50.0)
      (`TextRenderComponent.K2_SetText` (`self.Base Text`) (`KismetTextLibrary.Conv_StringToText` _outvalue))
      (`self.Get Turbine Cost`)
      (goto _label))))

(event `Get Turbine Cost`
  ;[1 1 1] Load Turbine Cost
  (bind (_outjsonobject _returnvalue) (`JsonBlueprintFunctionLibrary.FromString` (`/Game/Blueprints/BP_MQTT_Handler.Message` (`self.MQTT Handler`))))
  (if _returnvalue
    (bind (_outvalue _returnvalue_2) (`|GetJsonField` _outjsonobject "T1 Cost"))
    (if _returnvalue_2
      (`KismetSystemLibrary.PrintString` _outvalue false false (struct :`R` 1.0 :`G` 0.992648 :`B` 0.117468 :`A` 1.0) 50.0)
      (`BlueprintMapLibrary.Map_Add` (`self.Turbine Data`) "NewEnumerator9" _outvalue)
      (`self.Update UI` "NewEnumerator9" _outvalue)
      (set `self.Cost` _outvalue)
      (else
        (`KismetSystemLibrary.PrintString` "nooooooo" :!label _label_2)))
    (else
      (goto _label_2))))

(event `Update Turbine Info`)

(event `Get Turbine Power`
  ;[1 1 1] Load Turbine Data
  (bind (_outjsonobject _returnvalue) (`JsonBlueprintFunctionLibrary.FromString` (`/Game/Blueprints/BP_MQTT_Handler.Message` (`self.MQTT Handler`))))
  (if _returnvalue
    (bind (_outvalue _returnvalue_2) (`|GetJsonField` _outjsonobject (`KismetStringLibrary.Concat_StrStr` (`self.Turbine number`) " Power")))
    (if _returnvalue_2
      (`KismetSystemLibrary.PrintString` _outvalue false false (struct :`R` 1.0 :`G` 0.992648 :`B` 0.117468 :`A` 1.0) 50.0)
      (`BlueprintMapLibrary.Map_Add` (`self.Turbine Data`) "NewEnumerator10" _outvalue)
      (`self.Update UI` "NewEnumerator10" _outvalue)
      (set `self.Power` _outvalue)
      (else
        (`KismetSystemLibrary.PrintString` "nooooooo" :!label _label_3)))
    (else
      (goto _label_3))))

(event `Get Moring Line Failure`
  ;[1 1 1] Load Moring Line Failure
  (bind (_outjsonobject _returnvalue) (`JsonBlueprintFunctionLibrary.FromString` (`/Game/Blueprints/BP_MQTT_Handler.Message` (`self.MQTT Handler`))))
  (if _returnvalue
    (bind (_outvalue _returnvalue_2) (`|GetJsonField` _outjsonobject (`KismetStringLibrary.Concat_StrStr` (`self.Turbine number`) " g3")))
    (if _returnvalue_2
      (`KismetSystemLibrary.PrintString` _outvalue false false (struct :`R` 1.0 :`G` 0.992648 :`B` 0.117468 :`A` 1.0) 50.0)
      (`BlueprintMapLibrary.Map_Add` (`self.Turbine Data`) "NewEnumerator6" _outvalue)
      (`self.Update UI` "NewEnumerator6" _outvalue)
      (set `self.PF_Moring Line` _outvalue)
      (else
        (`KismetSystemLibrary.PrintString` "nooooooo" :!label _label_4)))
    (else
      (goto _label_4))))

(event `Get Tower Buckling`
  ;[1 1 1] Load Tower Buckling
  (bind (_outjsonobject _returnvalue) (`JsonBlueprintFunctionLibrary.FromString` (`/Game/Blueprints/BP_MQTT_Handler.Message` (`self.MQTT Handler`))))
  (if _returnvalue
    (bind (_outvalue _returnvalue_2) (`|GetJsonField` _outjsonobject (`KismetStringLibrary.Concat_StrStr` (`self.Turbine number`) " g1")))
    (if _returnvalue_2
      (`KismetSystemLibrary.PrintString` _outvalue false false (struct :`R` 1.0 :`G` 0.992648 :`B` 0.117468 :`A` 1.0) 50.0)
      (`BlueprintMapLibrary.Map_Add` (`self.Turbine Data`) "NewEnumerator4" _outvalue)
      (`self.Update UI` "NewEnumerator4" _outvalue)
      (set `self.PF_TBuckling` _outvalue)
      (else
        (`KismetSystemLibrary.PrintString` "nooooooo" :!label _label_5)))
    (else
      (goto _label_5))))

(event `Get Blade Root Bending`
  ;[1 1 1] Load Tower Buckling
  (bind (_outjsonobject _returnvalue) (`JsonBlueprintFunctionLibrary.FromString` (`/Game/Blueprints/BP_MQTT_Handler.Message` (`self.MQTT Handler`))))
  (if _returnvalue
    (bind (_outvalue _returnvalue_2) (`|GetJsonField` _outjsonobject (`KismetStringLibrary.Concat_StrStr` (`self.Turbine number`) " g2")))
    (if _returnvalue_2
      (`KismetSystemLibrary.PrintString` _outvalue false false (struct :`R` 1.0 :`G` 0.992648 :`B` 0.117468 :`A` 1.0) 50.0)
      (`BlueprintMapLibrary.Map_Add` (`self.Turbine Data`) "NewEnumerator5" _outvalue)
      (`self.Update UI` "NewEnumerator5" _outvalue)
      (set `self.PF_BRB` _outvalue)
      (else
        (`KismetSystemLibrary.PrintString` "No Tower Buckling" :!label _label_6)))
    (else
      (goto _label_6))))

(fn `UserConstructionScript`
  (bind _returnvalue (`KismetMathLibrary.Conv_IntToDouble` (`self.Height`)))
  (bind _returnvalue_2 (- _returnvalue 100.0))
  (bind _returnvalue_3 (+ (* _returnvalue_2 1.06) 105.0))
  ;[1 1 1] random rotor initial rotation
  (`SceneComponent.K2_AddLocalRotation` (`self.Rotor`) (`KismetMathLibrary.MakeRotator` 0.0 (`KismetMathLibrary.RandomFloatInRange` 0.0 360.0)) false false)
  ;[1 1 1] change logo
  (bind _returnvalue_4 (`KismetMaterialLibrary.CreateDynamicMaterialInstance` "/Game/Wind_Turbine/Materials/M_Wind_Turbine_logo.M_Wind_Turbine_logo"))
  (`PrimitiveComponent.SetMaterial` (`self.logo`) 0 _returnvalue_4)
  (`MaterialInstanceDynamic.SetTextureParameterValue` _returnvalue_4 "logo" (`self.Logo_texture`))
  ;[1 1 1] change height
  (`SceneComponent.SetRelativeScale3D` (`self.Pillar`) (`KismetMathLibrary.MakeVector` 1.0 1.0 (/ _returnvalue_3 100.0)))
  (`SceneComponent.K2_AddLocalOffset` (`self.Pillar`) (`KismetMathLibrary.MakeVector` 0.0 0.0 (+ (/ _returnvalue_3 -3.0) 30.0)) false false)
  (`SceneComponent.K2_AddLocalOffset` (`self.Nacelle`) (`KismetMathLibrary.MakeVector` 0.0 0.0 (* _returnvalue_2 100.0)) false false)
  (`MeshComponent.SetScalarParameterValueOnMaterials` (`self.Pillar`) "uv_height" _returnvalue)
  ;[1 1 1] change rotor diameter
  (`SceneComponent.SetRelativeScale3D` (`self.Rotor`) (`KismetMathLibrary.Conv_DoubleToVector` (/ (`self.Rotor diameter`) 80.0)))
  ;[1 1 1] Dirtiness
  (`MeshComponent.SetScalarParameterValueOnMaterials` (`self.Anemometer`) "Dirtiness" (`self.Dirtiness`))
  (`MeshComponent.SetScalarParameterValueOnMaterials` (`self.Base`) "Dirtiness" (`self.Dirtiness`))
  (`MeshComponent.SetScalarParameterValueOnMaterials` (`self.Pillar`) "Dirtiness" (`self.Dirtiness`))
  (`MeshComponent.SetScalarParameterValueOnMaterials` (`self.Nacelle`) "Dirtiness" (`self.Dirtiness`))
  (`MeshComponent.SetScalarParameterValueOnMaterials` (`self.Rotor`) "Dirtiness" (`self.Dirtiness`))
  ;[1 1 1] random speed
  (set `self.random_speed_change` (`KismetMathLibrary.RandomFloatInRange` -0.3 0.3))
  ;[1 1 1] Offshore
  (if (`self.Offshore Wind Turbine`)
    (`SceneComponent.K2_AddWorldOffset` (`self.Base`) (0.0 0.0 1650.0) false false)
    (else
      (`ActorComponent.K2_DestroyComponent` (`self.Offshore_base`))))
  (`ActorComponent.SetAutoActivate` (`self.Audio`) (`self.Sound`)))