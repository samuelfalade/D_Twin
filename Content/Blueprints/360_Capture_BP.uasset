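; 360 capture actor that renders its surroundings into a 2:1 panorama and exports it to disk as a numbered image sequence.
; On BeginPlay, if enabled with a save path, each SceneCaptureComponent2D gets a render target bound to the panorama material parameter matching its component name.
; While Capture is set, each Tick draws that material into the panorama target and exports it in the CaptureMode's HDR, JPG or PNG format.
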(event `self.ReceiveBeginPlay`
  (bind (_width _height) (`self.GetPanoMapResolution`))
  (bind (_width_2 _height_2) (`self.GetCaptureResolution`))
  (bind _capturemode (`self.CaptureMode`))
  (bind _returnvalue (select `byte` _capturemode :`0` "RTF_R8" :`1` "RTF_R8" :`2` "RTF_R8" :!type "ETextureRenderTargetFormat Enum"))
  ;[0.1 0.1 0.1] Capture Initialization
  (if (`self.bEnabled`)
    (if (`self.IsSavePathValid`)
      (`|ExecutionSequence`
        (:`then_0`
          (bind _returnvalue_2 (`KismetMaterialLibrary.CreateDynamicMaterialInstance` (`self.PanoMapMtl`)))
          (set `self.PanoMapDMI` _returnvalue_2)
          (bind _returnvalue_3 (`KismetRenderingLibrary.CreateRenderTarget2D` _width _height _returnvalue (struct)))
          (set `self.PanoMapRT` _returnvalue_3))
        (:`then_1`
          (for _array_element (`self.K2_GetComponentsByClass` "/Script/Engine.SceneCaptureComponent2D")
            (set `SceneCaptureComponent.CaptureSource` (select `byte` _capturemode :`0` "SCS_SceneColorHDR" :`1` "SCS_SceneColorHDR" :`2` "SCS_SceneColorHDR" :!type "ESceneCaptureSource Enum") _array_element)
            (bind _returnvalue_4 (`KismetRenderingLibrary.CreateRenderTarget2D` _width_2 _height_2 _returnvalue))
            (set `TextureRenderTarget.TargetGamma` (select `byte` _capturemode :`0` 0.0 :`1` 0.0 :`2` 0.0) _returnvalue_4)
            (bind _output_get (set `SceneCaptureComponent2D.TextureTarget` _returnvalue_4 _array_element))
            (`MaterialInstanceDynamic.SetTextureParameterValue` (`self.PanoMapDMI`) (`KismetStringLibrary.Conv_StringToName` (`KismetSystemLibrary.GetObjectName` _array_element)) _output_get)
            (set `SceneCaptureComponent.bCaptureEveryFrame` true _array_element))))
      (else
        (`KismetSystemLibrary.PrintString` "Warning: No output path selected" true true (struct :`R` 1.0 :`B` 0.096044 :`A` 1.0))))))

(event `self.ReceiveTick`
  (params (DeltaSeconds :type "Float (single-precision)"))
  (bind _panomaprt (`self.PanoMapRT`))
  ;[0.1 0.1 0.1] Frame Capture
  (if (`self.bCapture`)
    (`KismetRenderingLibrary.DrawMaterialToRenderTarget` _panomaprt (`self.PanoMapDMI`))
    (`ImageWriteBlueprintLibrary.ExportToDisk` _panomaprt (`self.GetFilePath`) (select `byte` (`self.CaptureMode`) :`0` (`self.ExportOptionsHDR`) :`1` (`self.ExportOptionsLDRJPG`) :`2` (`self.ExportOptionsLDRPNG`)))
    (`/Engine/EditorBlueprintResources/StandardMacros.IncrementInt` (`self.FirstFrameNumber`))))

(fn `GetCaptureResolution`
  (returns (Width :type Integer) (Height :type Integer))
  (bind _returnvalue (select `byte` (`self.CaptureResolution`) :`0` 0 :`1` 0 :`2` 0 :`3` 0 :`4` 0 :`5` 0))
  (return _returnvalue _returnvalue))

(fn `GetFilePath`
  (returns (ReturnValue :type String))
  (bind _savepath_path (break `DirectoryPath` (`self.SavePath`)))
  (return (`KismetStringLibrary.BuildString_Name` (`KismetStringLibrary.Concat_StrStr` _savepath_path "\\") (`KismetStringLibrary.Concat_StrStr` (`self.FileName`) "_") (`KismetStringLibrary.Conv_StringToName` (`KismetStringLibrary.Right` (`KismetStringLibrary.Concat_StrStr` "000" (`KismetStringLibrary.Conv_IntToString` (`self.FirstFrameNumber`))) 4)))))

(fn `GetPanoMapResolution`
  (returns (Width :type Integer) (Height :type Integer))
  (bind _returnvalue (select `byte` (`self.CaptureResolution`) :`0` 0 :`1` 0 :`2` 0 :`3` 0 :`4` 0 :`5` 0))
  (return (* _returnvalue 2) _returnvalue))

(fn `IsSavePathValid`
  (returns (ReturnValue :type Boolean))
  (bind _savepath_path (break `DirectoryPath` (`self.SavePath`)))
  (return (not (<= (`KismetStringLibrary.Len` _savepath_path) 0))))

(fn `UserConstructionScript`)