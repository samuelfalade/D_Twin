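; Actor that connects to an MQTT broker and feeds live wind turbine telemetry to the UI.
; BeginPlay creates the client, connects, subscribes to the "Turbine" topic, publishes an empty message and binds handlers.
; Each received message is parsed as JSON by per-field events, which store values in TurbineData and fire CallUpdateUI.
; MeanWindSpeed duplicates WaveHeight's field and key, while PowerGeneration builds its field name from FieldName plus "g1".
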(event `Connect Callback`
  ;[1 1 1] Connect to MQTT server
  (`KismetSystemLibrary.PrintString` "Connected" false false (struct :`G` 0.66 :`B` 1.0 :`A` 1.0) 20.0))

(event `Subscribe Callback`
  (params (mid :type Integer) (qos :type "Array of Integer (by ref)"))
  ;[1 1 1] Subscribe to message
  (`KismetSystemLibrary.PrintString` "Subscribed" true true (struct :`R` 1.0 :`G` 0.286385 :`B` 0.226637 :`A` 1.0) 20.0))

(event `self.ReceiveBeginPlay`
  (bind _mqtt_client (`self.MQTT Client`))
  (`|ExecutionSequence`
    (:`then_0`
      ;[1 1 1] Create Client
      (bind _returnvalue (`MqttUtilitiesBPL.CreateMqttClient` (make `MqttClientConfig` "datahub.tamids.tamu.edu" 1883 "Unreal_Client")))
      (set `self.MQTT Client` _returnvalue))
    (:`then_1`
      ;[1 1 1] Connect to MQTT server
      (`MqttClientInterface.Connect` :`self` (`self.MQTT Client`) :`onConnectCallback` (delegate `Connect Callback`)))
    (:`then_2`
      ;[1 1 1] Subscribe to message
      (`MqttClientInterface.Subscribe` _mqtt_client "Turbine" 0)
      (`MqttClientInterface.SetOnSubscribeHandler` _mqtt_client (delegate `Subscribe Callback`)))
    (:`then_3`
      ;[1 1 1] Publish Message
      (`MqttClientInterface.Publish` (`self.MQTT Client`) (make `MqttMessage` "")))
    (:`then_4`
      ;[1 1 1] Message Handler
      (`MqttClientInterface.SetOnMessageHandler` (`self.MQTT Client`) (delegate `Message Recieved`)))
    (:`then_5`
      ;[1 1 1] Handle Errors
      (`MqttClientInterface.SetOnErrorHandler` (`self.MQTT Client`) (delegate `On Error Callback`)))))

(event `Message Recieved`
  (params (message :type "MqttMessage Structure"))
  (bind (_message _topic) (break `MqttMessage` message))
  ;[1 1 1] Message Handler
  (`KismetSystemLibrary.PrintString` (`KismetStringLibrary.Concat_StrStr` "" _message) false false (struct :`R` 0.067723 :`G` 1.0 :`B` 0.21626 :`A` 1.0) 20.0)
  (`KismetSystemLibrary.PrintString` (`KismetStringLibrary.Concat_StrStr` _topic) false false (struct :`R` 1.0 :`G` 0.054146 :`B` 0.89767 :`A` 1.0) 20.0)
  (bind _output_get (set `self.Message` _message))
  ;[0.4187 0.6488 1] Publish to UI
  ;;[1 1 1] Mine data
  (`self.Power Generation`)
  (`self.Mean Wind Speed`)
  (`self.Time`)
  (`self.Wave Height`)
  (`self.Wind Speed`)
  (`self.Total Power`))

(event `Total Power`
  ;[0.4187 0.6488 1] Publish to UI
  ;;[1 1 1] Total Power
  (bind (_outjsonobject _returnvalue) (`JsonBlueprintFunctionLibrary.FromString` (stale `Message Recieved` _output_get)))
  (if _returnvalue
    (bind (_outvalue _returnvalue_2) (`|GetJsonField` _outjsonobject "Total Power"))
    (if _returnvalue_2
      (`KismetSystemLibrary.PrintString` _outvalue false false (struct :`R` 1.0 :`G` 0.992648 :`B` 0.117468 :`A` 1.0) 50.0)
      (`BlueprintMapLibrary.Map_Add` (`self.Turbine Data`) "NewEnumerator1" _outvalue)
      (`self.Update UI` "NewEnumerator1" _outvalue))))

(event `On Error Callback`
  (params (code :type Integer) (message :type String))
  ;[1 1 1] Handle Errors
  (`KismetSystemLibrary.PrintString` (`KismetStringLibrary.Concat_StrStr` "Error - Code: " (`KismetStringLibrary.Conv_IntToString` code) "Message: " message) false false (struct :`R` 0.408935 :`G` 0.012508 :`B` 0.583333 :`A` 1.0) 20.0))

(event `Wind Speed`
  ;[0.4187 0.6488 1] Publish to UI
  ;;[1 1 1] Wind Speed
  (bind (_outjsonobject _returnvalue) (`JsonBlueprintFunctionLibrary.FromString` (stale `Message Recieved` _output_get)))
  (if _returnvalue
    (bind (_outvalue _returnvalue_2) (`|GetJsonField` _outjsonobject "Wind Speed"))
    (if _returnvalue_2
      (`KismetSystemLibrary.PrintString` _outvalue false false (struct :`R` 1.0 :`G` 0.992648 :`B` 0.117468 :`A` 1.0) 50.0)
      (`BlueprintMapLibrary.Map_Add` (`self.Turbine Data`) "NewEnumerator2" _outvalue)
      (`self.Update UI` "NewEnumerator2" _outvalue))))

(event `Wave Height`
  ;[0.4187 0.6488 1] Publish to UI
  ;;[1 1 1] Wave Height
  (bind (_outjsonobject _returnvalue) (`JsonBlueprintFunctionLibrary.FromString` (stale `Message Recieved` _output_get)))
  (if _returnvalue
    (bind (_outvalue _returnvalue_2) (`|GetJsonField` _outjsonobject "Wave Height"))
    (if _returnvalue_2
      (`KismetSystemLibrary.PrintString` _outvalue false false (struct :`R` 1.0 :`G` 0.992648 :`B` 0.117468 :`A` 1.0) 50.0)
      (`BlueprintMapLibrary.Map_Add` (`self.Turbine Data`) "NewEnumerator3" _outvalue)
      (`self.Update UI` "NewEnumerator3" _outvalue))))

(event `Time`
  ;[0.4187 0.6488 1] Publish to UI
  ;;[1 1 1] xxxxxxx
  (bind (_outjsonobject _returnvalue) (`JsonBlueprintFunctionLibrary.FromString` (stale `Message Recieved` _output_get)))
  (if _returnvalue
    (bind (_outvalue _returnvalue_2) (`|GetJsonField` _outjsonobject "Time"))
    (if _returnvalue_2
      (`KismetSystemLibrary.PrintString` _outvalue false false (struct :`R` 1.0 :`G` 0.992648 :`B` 0.117468 :`A` 1.0) 50.0)
      (`BlueprintMapLibrary.Map_Add` (`self.Turbine Data`) "NewEnumerator0" _outvalue)
      (`self.Update UI` "NewEnumerator0" _outvalue))))

(event `Mean Wind Speed`
  ;[0.4187 0.6488 1] Publish to UI
  ;;[1 1 1] Mean Wind Speed
  (bind (_outjsonobject _returnvalue) (`JsonBlueprintFunctionLibrary.FromString` (stale `Message Recieved` _output_get)))
  (if _returnvalue
    (bind (_outvalue _returnvalue_2) (`|GetJsonField` _outjsonobject "Wave Height"))
    (if _returnvalue_2
      (`KismetSystemLibrary.PrintString` _outvalue false false (struct :`R` 1.0 :`G` 0.992648 :`B` 0.117468 :`A` 1.0) 50.0)
      (`BlueprintMapLibrary.Map_Add` (`self.Turbine Data`) "NewEnumerator3" _outvalue)
      (`self.Update UI` "NewEnumerator3" _outvalue))))

(event `Power Generation`
  ;[0.4187 0.6488 1] Publish to UI
  ;;[1 1 1] Power Generation
  (bind (_outjsonobject _returnvalue) (`JsonBlueprintFunctionLibrary.FromString` (stale `Message Recieved` _output_get)))
  (if _returnvalue
    (bind (_outvalue _returnvalue_2) (`|GetJsonField` _outjsonobject (`KismetStringLibrary.Concat_StrStr` (`self.Field Name`) " g1")))
    (if _returnvalue_2
      (`KismetSystemLibrary.PrintString` _outvalue false false (struct :`R` 1.0 :`G` 0.992648 :`B` 0.117468 :`A` 1.0) 50.0)
      (`BlueprintMapLibrary.Map_Add` (`self.Turbine Data`) "NewEnumerator4" _outvalue)
      (`self.Update UI` "NewEnumerator4" _outvalue))))

(fn `UserConstructionScript`)